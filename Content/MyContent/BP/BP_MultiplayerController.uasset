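; BP_MultiplayerController is a controller that turns every character's health widget toward the local player's camera.
; Each Tick it casts player character 0 to BP_MultiplayerCharacter and caches that camera's location.
; It then finds all BP_MultiplayerCharacter actors with GetAllActorsOfClass, every frame.
; Each one's health component and location go to the local character's SetRotationHealthToCamera, which handles the rotation.
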(event `self.ReceiveTick`
  (params (DeltaSeconds :type "Float (single-precision)"))
  (`self.UpdateRotationHealth`))

(event `UpdateRotationHealth`
  (bind _asbp_multiplayer_character (cast `/Game/MyContent/BP/BP_MultiplayerCharacter` (`GameplayStatics.GetPlayerCharacter` 0)))
  (set `self.CurCharacter` _asbp_multiplayer_character)
  (`|ExecutionSequence`
    (:`then_0`
      (bind _cameralocation (`/Game/MyContent/BP/BP_MultiplayerCharacter.GetCameraLocation` (`self.CurCharacter`)))
      (set `self.PlayerCameraLocataion` _cameralocation))
    (:`then_1`
      (bind _outactors (`GameplayStatics.GetAllActorsOfClass` "/Game/MyContent/BP/BP_MultiplayerCharacter.BP_MultiplayerCharacter_C"))
      (for _array_element _outactors
        (bind _healthcomponentlocation (`/Game/MyContent/BP/BP_MultiplayerCharacter.GetHealthComponentLocation` _array_element))
        (bind _healthcomponent (`/Game/MyContent/BP/BP_MultiplayerCharacter.GetHealthComponent` _array_element))
        (`/Game/MyContent/BP/BP_MultiplayerCharacter.SetRotationHealthToCamera` (`self.CurCharacter`) (`self.PlayerCameraLocataion`) _healthcomponentlocation _healthcomponent)))))

(fn `UserConstructionScript`)