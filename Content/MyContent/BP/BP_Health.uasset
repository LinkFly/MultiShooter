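; BP_Health is a health Blueprint that tracks damage and reports whether its owner is alive.
; Init stores a health widget reference and sets Health to InitHealth, and TakeDamage subtracts damage without clamping.
; Health's RepNotify prints the value and updates the widget's percentage against MaxHealth.
; IsLife returns false only when Health is nearly zero, so negative health still counts as alive.
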(fn `Init`
  (params (HealthWidget :type "/Game/MyContent/Widgets/WBP_Health Object Reference"))
  (set `self.HealthWidget` HealthWidget)
  (set `self.Health` (`self.InitHealth`)))

(fn `IsLife`
  (returns (bLife :type Boolean))
  (return (not (`KismetMathLibrary.NearlyEqual_FloatFloat` (`self.Health`)))))

(fn `OnRep_Health`
  (`KismetSystemLibrary.PrintString` (`KismetStringLibrary.Concat_StrStr` "Health: " (`KismetStringLibrary.Conv_DoubleToString` (`self.Health`))))
  (`/Game/MyContent/Widgets/WBP_Health.UpdatePercent` (`self.HealthWidget`) (`self.Health`) (`self.MaxHealth`)))

(fn `TakeDamage`
  (params (Damage :type "Float (double-precision)"))
  (set `self.Health` (- (`self.Health`) Damage))
  (return))