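; BP_Projectile is a multiplayer projectile that flies forward, damages characters and explodes on impact.
; The server moves it each tick without sweep and handles sphere overlaps, ignoring the owner, damaging BP_MultiplayerCharacter and ending other projectiles it hits.
; A multicast spawns the explosion, hides the projectile and disables its collision.
; It is destroyed when the explosion finishes or its lifetime timer expires.
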(event `self.ReceiveBeginPlay`
  (`KismetSystemLibrary.K2_SetTimerDelegate` (delegate `LifeEnded`) (`self.TTL`)))

(event `LifeEnded`
  (`self.Server_LifeEnded`))

(event `Server_LifeEnded`
  (`KismetSystemLibrary.Delay` 0.0)
  (`self.K2_DestroyActor`))

(event `Server_Move`
  (params (DeltaTime :type "Float (double-precision)"))
  (`self.K2_SetActorLocation` (+ (* (`self.GetActorForwardVector`) (* DeltaTime (`self.Speed`))) (`self.K2_GetActorLocation`))))

(event `self.ReceiveTick`
  (params (DeltaSeconds :type "Float (single-precision)"))
  (if (`KismetSystemLibrary.IsServer`)
    (`self.Server_Move` DeltaSeconds)))

(event `self.Sphere1.OnComponentBeginOverlap`
  (params (OverlappedComponent :type "PrimitiveComponent Object Reference") (OtherActor :type "Actor Object Reference") (OtherComp :type "PrimitiveComponent Object Reference") (OtherBodyIndex :type Integer) (bFromSweep :type Boolean) (SweepResult :type "HitResult Structure (by ref)"))
  (if (and (`KismetSystemLibrary.IsServer`) (!= OtherActor self))
    (`self.Server_Collision` OtherActor (`self.K2_GetActorLocation`))))

(event `Server_Collision`
  (params (OtherActor :type "Actor Object Reference") (Location :type "Vector Structure"))
  (if (!= OtherActor (`self.GetOwner`))
    (bind _asbp_multiplayer_character (cast `/Game/MyContent/BP/BP_MultiplayerCharacter` OtherActor)
      (:`then`
        (`/Game/MyContent/BP/BP_MultiplayerCharacter.Server_TakeDamage` _asbp_multiplayer_character (`self.Damage`)))
      (:`CastFailed`
        (bind _asbp_projectile (cast `/Game/MyContent/BP/BP_Projectile` OtherActor)
          (:`then`
            (`self.Server_LifeEnded` _asbp_projectile))
          (:`CastFailed`
            _))))
    (`self.MulticastHitEffect` (`self.K2_GetActorLocation`))))

(event `SpawnHitEffect`
  (params (HitLocation :type "Vector Structure"))
  (bind _returnvalue (`GameplayStatics.SpawnEmitterAtLocation` "/Game/StarterContent/Particles/P_Explosion.P_Explosion" HitLocation))
  (`SceneComponent.SetVisibility` (`self.DefaultSceneRoot`) false true)
  (`self.SetActorEnableCollision` false)
  (add `ParticleSystemComponent.OnSystemFinished` _returnvalue (delegate `OnSystemFinished_Event_0`)))

(event `OnSystemFinished_Event_0`
  (params (PSystem :type "ParticleSystemComponent Object Reference"))
  (`self.Server_LifeEnded`))

(event `MulticastHitEffect`
  (params (HitLocation :type "Vector Structure"))
  (`self.SpawnHitEffect` HitLocation))

(fn `UserConstructionScript`)