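; Game instance that hosts, lists and joins LAN multiplayer sessions and reports network failures on screen.
; CreateGame creates a LAN session, then opens Level1 as a listen server.
; GetGames prints found servers with player counts and ping, while JoinToGame searches for a single result and joins it directly.
; Session failures, network errors and travel errors appear only as printed debug messages.
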(event `CreateGame`
  (`CreateSessionCallbackProxy.CreateSession` (`GameplayStatics.GetPlayerController` 0) 16 true
    (:`OnSuccess`
      (`GameplayStatics.OpenLevel` "Level1" true "listen"))
    (:`OnFailure`
      (`KismetSystemLibrary.PrintString` "Game create error!" true true (struct :`G` 0.66 :`B` 1.0 :`A` 1.0) 10.0))))

(event `GetGames`
  (bind _results (`FindSessionsCallbackProxy.FindSessions` (`GameplayStatics.GetPlayerController` 0) 20 true)
    (:`OnSuccess`
      (for _array_element _results
        (`KismetSystemLibrary.PrintString` (`KismetStringLibrary.Concat_StrStr` "Server: " (`FindSessionsCallbackProxy.GetServerName` _array_element) " \nPlayers: " (`KismetStringLibrary.Conv_IntToString` (`FindSessionsCallbackProxy.GetCurrentPlayers` _array_element)) " / " (`KismetStringLibrary.Conv_IntToString` (`FindSessionsCallbackProxy.GetMaxPlayers` _array_element)) " \nPing: " (`KismetStringLibrary.Conv_IntToString` (`FindSessionsCallbackProxy.GetPingInMs` _array_element))) true true (struct :`G` 0.66 :`B` 1.0 :`A` 1.0) 30.0)))
    (:`OnFailure`
      (`KismetSystemLibrary.PrintString` "Not found sessions" true true (struct :`G` 0.66 :`B` 1.0 :`A` 1.0) 5.0))))

(event `JoinToGame`
  (bind _results (`FindSessionsCallbackProxy.FindSessions` (`GameplayStatics.GetPlayerController` 0) 1 true)
    (:`OnSuccess`
      (for _array_element _results
        (`JoinSessionCallbackProxy.JoinSession` (`GameplayStatics.GetPlayerController` 0) _array_element
          (:`OnFailure`
            (`KismetSystemLibrary.PrintString` "ERROR!!! Join session" true true (struct :`R` 1.0 :`G` 0.024056 :`A` 1.0) 5.0)))))
    (:`OnFailure`
      (`KismetSystemLibrary.PrintString` "Not found sessions" true true (struct :`G` 0.66 :`B` 1.0 :`A` 1.0) 5.0))))

(event `self.HandleNetworkError`
  (params (FailureType :type "ENetworkFailure Enum" :default "NetDriverAlreadyExists") (bIsServer :type Boolean))
  (`KismetSystemLibrary.PrintString` (`KismetStringLibrary.Concat_StrStr` "Network error!" "Failure type: " (`|GetEnumeratorNameAsString` FailureType) "On Server: " (`KismetStringLibrary.Conv_BoolToString` bIsServer)) true true (struct :`R` 1.0 :`G` 0.058691 :`A` 1.0) 20.0))

(event `self.HandleTravelError`
  (params (FailureType :type "ETravelFailure Enum" :default "NoLevel"))
  (`KismetSystemLibrary.PrintString` (`|GetEnumeratorNameAsString` FailureType) true true (struct :`R` 1.0 :`G` 0.058691 :`A` 1.0) 20.0))